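; Stealth-game enemy AI character that patrols, investigates noises, chases the player and makes melee attacks.
; Tick uses movement flags and PlayerVisible to choose chase or random patrol, while PawnSensing sight and hearing trigger chase and investigation through AIMoveTo.
; Reaching the player plays an attack montage whose notify sphere-traces from the right hand and reloads a hit player's checkpoint.
; Waypoint patrol is uncalled here, with an empty next-point function.
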(event OnSeePawn(PawnSensing)
  (params (Pawn :type Pawn%20Object%20Reference))
  (if (Actor|ActorHasTag Pawn "Player")
    (CallFunction|ChasePlayer Pawn)))

(event Custom|ChasePlayer
  (params (Pawn :type Pawn%20Object%20Reference))
  (CallFunction|UpdateWalkSpeed 4e+02)
  (Variables|Default|SetbCanMove false)
  (Variables|Default|SetbCanChase false)
  (AI|AIMoveTo self "0, 0, 0" (Game|Player|GetPlayerPawn 0) 5.0 false
    (:OnSuccess
      (CallFunction|Attack))
    (:OnFail
      _))
  (Utilities|FlowControl|Delay 3.0)
  (Variables|Default|SetbCanMove true)
  (Variables|Default|SetbCanChase true))

(event Custom|Attack
  (bind _mesh (Variables|Character|GetMesh))
  (bind _returnvalue (Transformation|GetSocketLocation _mesh "hand_r"))
  ;[0.15 0.15 0.15 0.5] Melee Attack
  (Utilities|FlowControl|DoOnce false
    (:Completed
      (bind _notifyname (Animation|Montage|PlayMontage (Variables|Character|GetMesh) "/Game/StealthGame/Characters/Enemies/AM_Attack_01.AM_Attack_01")
        (:OnCompleted
          (CallFunction|ResetAttack))
        (:OnNotifyBegin
          (switch name _notifyname
            (:AttackDamage
              (Development|PrintString "I got you now!")
              (bind (_outhits _returnvalue_2) (Collision|MultiSphereTraceForObjects _returnvalue (+ _returnvalue (* (Transformation|GetActorForwardVector) (Variables|Default|GetMeleeTraceDistance))) (Variables|Default|GetMeleeTraceRadius) (Utilities|Array|MakeArray "ObjectTypeQuery3") false 0 "ForOneFrame"))
              (if _returnvalue_2
                (for _array_element _outhits
                  (bind _asbp_third_person_character_custom (Utilities|Casting|CastToBP_ThirdPersonCharacterCustom (.HitActor (Collision|BreakHitResult _array_element))))
                  (Default|LoadCheckpoint _asbp_third_person_character_custom))))))))))

(event Custom|ResetAttack
  (bind _mesh (Variables|Character|GetMesh))
  (bind _returnvalue (Transformation|GetSocketLocation _mesh "hand_r"))
  ;[0.15 0.15 0.15 0.5] Melee Attack
  (Utilities|FlowControl|DoOnce false) ; enters at Reset
)

(event Custom|RandomPatrol
  (CallFunction|UpdateWalkSpeed 2e+02)
  (Variables|Default|SetbCanMove false)
  (AI|AIMoveTo self (.RandomLocation (AI|Navigation|GetRandomReachablePointinRadius (Transformation|GetActorLocation) 2e+03 0 0)) 0 3e+01 false
    (:OnSuccess
      (Utilities|FlowControl|Delay 2.0)
      (Variables|Default|SetbCanMove true))))

(event Custom|MoveToNextTargetPoint
  (CallFunction|UpdateWalkSpeed 2e+02)
  (Variables|Default|SetbCanMove false)
  (AI|AIMoveTo self "0, 0, 0" (Utilities|Array|Get(acopy) (Variables|Default|GetPatrolTargetPoints) (Variables|Default|GetCurrentIndex)) 5.0 false
    (:OnSuccess
      _)
    (:OnFail
      _))
  (Utilities|FlowControl|Delay 4.0)
  (CallFunction|GetNextPatrolPoint)
  (Variables|Default|SetbCanMove true))

(event EventBeginPlay)

(event Collision|EventActorBeginOverlap
  (params (OtherActor :type Actor%20Object%20Reference)))

(event EventTick
  (params (DeltaSeconds :type Float%20%28single-precision%29))
  (if (Variables|Default|GetbCanMove)
    (if (Variables|Default|GetbPlayerVisible)
      (CallFunction|ChasePlayer)
      (else
        (CallFunction|RandomPatrol)))
    (elif (and (Variables|Default|GetbPlayerVisible) (Variables|Default|GetbCanChase))
      (Components|Movement|StopMovementImmediately (Variables|Character|GetCharacterMovement))
      (CallFunction|ChasePlayer))))

(fn ConstructionScript)

(fn UpdateWalkSpeed
  (params (New%20Walk%20Speed :type Float%20%28double-precision%29))
  (Variables|/Script/Engine.CharacterMovementComponent|SetMaxWalkSpeed (Variables|Character|GetCharacterMovement) New%20Walk%20Speed))

(fn GetNextPatrolPoint)

(event OnHearNoise(PawnSensing)
  (params (Instigator :type Pawn%20Object%20Reference) (Location :type Vector%20%28by%20ref%29 :default "0, 0, 0") (Volume :type Float%20%28single-precision%29))
  (if (not (Variables|Default|GetbPlayerVisible))
    (Development|PrintString "What was that noise?")
    (CallFunction|UpdateWalkSpeed 275.0)
    (Variables|Default|SetbCanMove false)
    (AI|AIMoveTo self Location 0 5.0 false
      (:OnSuccess
        (Utilities|FlowControl|Delay 2e+01)
        (Variables|Default|SetbCanMove true)))))