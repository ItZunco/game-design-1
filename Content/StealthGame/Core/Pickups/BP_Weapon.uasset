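; BP_Weapon is a pickup weapon actor for the stealth game's custom third-person character.
; The first overlap of its trigger passes the weapon to the character's TryToPickUp and destroys its point light, with a DoOnce that is used up even by other actors.
; Pickup attaches the root to the given mesh's hand_r socket.
; Primary and secondary actions only print placeholder debug text.
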(event OnComponentBeginOverlap(PickupTrigger)
  (params (OverlappedComponent :type Primitive%20Component%20Object%20Reference) (OtherActor :type Actor%20Object%20Reference) (OtherComp :type Primitive%20Component%20Object%20Reference) (OtherBodyIndex :type Integer) (bFromSweep :type Boolean) (SweepResult :type Hit%20Result%20Structure%20%28by%20ref%29))
  (Utilities|FlowControl|DoOnce false
    (:Completed
      (Development|PrintString "Finally... a weapon." true true "(R=1.000000,G=0.000000,B=0.000000,A=1.000000)")
      (bind _asbp_third_person_character_custom (Utilities|Casting|CastToBP_ThirdPersonCharacterCustom OtherActor))
      (Default|TrytoPickUp _asbp_third_person_character_custom self)
      (Components|DestroyComponent (Variables|Default|GetPointLight)))))

(event EventBeginPlay)

(event Collision|EventActorBeginOverlap
  (params (OtherActor :type Actor%20Object%20Reference)))

(event EventTick
  (params (DeltaSeconds :type Float%20%28single-precision%29)))

(event EventPickup
  (params (ParentMesh :type Skeletal%20Mesh%20Component%20Object%20Reference))
  (Transformation|AttachComponentToComponent (Variables|Default|GetDefaultSceneRoot) ParentMesh "hand_r" "SnapToTarget" "KeepRelative" "KeepRelative" true))

(event EventPrimaryAction
  (params (ref_thirdPersonCharCustom :type BP%20Third%20Person%20Character%20Custom%20Object%20Reference))
  (Development|PrintString "DIE DIE DIE!!!" true true "(R=1.000000,G=0.000000,B=0.000000,A=1.000000)"))

(event EventSecondaryAction
  (Development|PrintString "BLOODSHED!!!" true true "(R=1.000000,G=0.000000,B=0.000000,A=1.000000)"))

(fn ConstructionScript)