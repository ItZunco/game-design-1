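; Stealth-game enemy AI character that roams, chases the player and dies by ragdolling when its capsule overlaps the player.
; PawnSensing sightings of Player-tagged pawns trigger a faster AIMoveTo chase.
; Tick uses movement and visibility flags to pick chase or random-point patrol, though PlayerVisible is never set here.
; Waypoint patrol is uncalled, and its next-point function is empty.
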(event OnComponentBeginOverlap(CapsuleComponent)
  (params (OverlappedComponent :type Primitive%20Component%20Object%20Reference) (OtherActor :type Actor%20Object%20Reference) (OtherComp :type Primitive%20Component%20Object%20Reference) (OtherBodyIndex :type Integer) (bFromSweep :type Boolean) (SweepResult :type Hit%20Result%20Structure%20%28by%20ref%29))
  (Utilities|Casting|CastToBP_ThirdPersonCharacterCustom OtherActor)
  (Physics|SetSimulatePhysics (Variables|Character|GetMesh) true)
  (Components|DestroyComponent (Variables|Collision|GetCapsuleComponent)))

(event OnSeePawn(PawnSensing)
  (params (Pawn :type Pawn%20Object%20Reference))
  (if (Actor|ActorHasTag Pawn "Player")
    (CallFunction|ChasePlayer Pawn)))

(event Custom|ChasePlayer
  (params (Pawn :type Pawn%20Object%20Reference))
  (CallFunction|UpdateWalkSpeed 4e+02)
  (Variables|Default|SetbCanMove false)
  (Variables|Default|SetbCanChase false)
  (AI|AIMoveTo self "0, 0, 0" (Game|Player|GetPlayerPawn 0) 5.0 false
    (:OnSuccess
      (Variables|Default|SetbCanMove true)
      (Variables|Default|SetbCanChase true))))

(event Custom|RandomPatrol
  (CallFunction|UpdateWalkSpeed 2e+02)
  (Variables|Default|SetbCanMove false)
  (AI|AIMoveTo self (.RandomLocation (AI|Navigation|GetRandomReachablePointinRadius (Transformation|GetActorLocation) 2e+03 0 0)) 0 3e+01 false
    (:OnSuccess
      (Utilities|FlowControl|Delay 2.0)
      (Variables|Default|SetbCanMove true))))

(event Custom|MoveToNextTargetPoint
  (CallFunction|UpdateWalkSpeed 2e+02)
  (Variables|Default|SetbCanMove false)
  (AI|AIMoveTo self "0, 0, 0" (Utilities|Array|Get(acopy) (Variables|Default|GetPatrolTargetPoints) (Variables|Default|GetCurrentIndex)) 5.0 false
    (:OnSuccess
      _)
    (:OnFail
      _))
  (Utilities|FlowControl|Delay 4.0)
  (CallFunction|GetNextPatrolPoint)
  (Variables|Default|SetbCanMove true))

(event EventBeginPlay)

(event Collision|EventActorBeginOverlap
  (params (OtherActor :type Actor%20Object%20Reference)))

(event EventTick
  (params (DeltaSeconds :type Float%20%28single-precision%29))
  (if (Variables|Default|GetbCanMove)
    (if (Variables|Default|GetbPlayerVisible)
      (CallFunction|ChasePlayer)
      (else
        (CallFunction|RandomPatrol)))
    (elif (and (Variables|Default|GetbPlayerVisible) (Variables|Default|GetbCanChase))
      (Components|Movement|StopMovementImmediately (Variables|Character|GetCharacterMovement))
      (CallFunction|ChasePlayer))))

(fn ConstructionScript)

(fn UpdateWalkSpeed
  (params (New%20Walk%20Speed :type Float%20%28double-precision%29))
  (Variables|/Script/Engine.CharacterMovementComponent|SetMaxWalkSpeed (Variables|Character|GetCharacterMovement) New%20Walk%20Speed))

(fn GetNextPatrolPoint)